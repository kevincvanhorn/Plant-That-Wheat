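; Fountain actor Blueprint that publishes its position and a sphere radius to the MPC_Fountain material parameter collection.
; The construction script and Tick both write the actor location to "Loc" and the SphereMask component's scaled radius to "Radius".
; This keeps any materials reading the collection in sync with the fountain, both in the editor and at runtime.
; The Bake function is an empty stub.
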(event EventBeginPlay)

(event Collision|EventActorBeginOverlap
  (params (OtherActor :type Actor%20Object%20Reference)))

(event EventTick
  (params (DeltaSeconds :type Float%20%28single-precision%29))
  (Rendering|Material|SetVectorParameterValue "/Game/Meshes/PDesert/Fountain/MPC_Fountain.MPC_Fountain" "Loc" (Math|Conversions|ToLinearColor(Vector) (Transformation|GetActorLocation)) :!class /Script/Engine.KismetMaterialLibrary)
  (Rendering|Material|SetScalarParameterValue "/Game/Meshes/PDesert/Fountain/MPC_Fountain.MPC_Fountain" "Radius" (Components|Sphere|GetScaledSphereRadius (Variables|Default|GetSphereMask)) :!class /Script/Engine.KismetMaterialLibrary))

(fn ConstructionScript
  (Rendering|Material|SetVectorParameterValue "/Game/Meshes/PDesert/Fountain/MPC_Fountain.MPC_Fountain" "Loc" (Math|Conversions|ToLinearColor(Vector) (Transformation|GetActorLocation)) :!class /Script/Engine.KismetMaterialLibrary)
  (Rendering|Material|SetScalarParameterValue "/Game/Meshes/PDesert/Fountain/MPC_Fountain.MPC_Fountain" "Radius" (Components|Sphere|GetScaledSphereRadius (Variables|Default|GetSphereMask)) :!class /Script/Engine.KismetMaterialLibrary))

(fn Bake)