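; BP_Hole is an actor that defines a spherical hole through the MPC_Opacity material parameter collection.
; It writes its location and the scaled radius of its SphereMask component to that collection on construction and every Tick.
; The construction script also calls Bake, which draws a hole material into a render target; Tick does not re-bake.
; Only one Location and Radius pair is stored, so multiple instances overwrite each other's values.
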(event EventBeginPlay)

(event Collision|EventActorBeginOverlap
  (params (OtherActor :type Actor%20Object%20Reference)))

(event EventTick
  (params (DeltaSeconds :type Float%20%28single-precision%29))
  (Rendering|Material|SetVectorParameterValue "/Game/Materials/Planet/PDesert/MPC_Opacity.MPC_Opacity" "Location" (Math|Conversions|ToLinearColor(Vector) (Transformation|GetActorLocation)) :!class /Script/Engine.KismetMaterialLibrary)
  (Rendering|Material|SetScalarParameterValue "/Game/Materials/Planet/PDesert/MPC_Opacity.MPC_Opacity" "Radius" (Components|Sphere|GetScaledSphereRadius (Variables|Default|GetSphereMask)) :!class /Script/Engine.KismetMaterialLibrary))

(fn ConstructionScript
  (Rendering|Material|SetVectorParameterValue "/Game/Materials/Planet/PDesert/MPC_Opacity.MPC_Opacity" "Location" (Math|Conversions|ToLinearColor(Vector) (Transformation|GetActorLocation)) :!class /Script/Engine.KismetMaterialLibrary)
  (Rendering|Material|SetScalarParameterValue "/Game/Materials/Planet/PDesert/MPC_Opacity.MPC_Opacity" "Radius" (Components|Sphere|GetScaledSphereRadius (Variables|Default|GetSphereMask)) :!class /Script/Engine.KismetMaterialLibrary)
  (CallFunction|Bake))

(fn Bake
  (Rendering|DrawMaterialtoRenderTarget "/Game/Materials/Planet/PDesert/Sand/RT_Approach/Try_3/RT_Hole_5.RT_Hole_5" "/Game/Materials/Planet/PDesert/Sand/RT_Approach/Try_3/Mat_RT_Holes_2.Mat_RT_Holes_2"))