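; Wheat seedling actor that animates its response to healthy spawn, unhealthy spawn and being fully watered.
; BeginPlay caches the base scale and creates a dynamic material, then timelines scale the actor for each event.
; Unhealthy spawn also plays a shrivel animation, tints the top color and flags the actor ready to destroy.
; Full watering randomizes the target scale per axis and rescales the seedling mesh, then hides it and disables its collision.
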(event EventBeginPlay
  (bind _skeletalmesh (Variables|Default|GetSkeletalMesh))
  (bind _returnvalue (Rendering|Material|CreateDynamicMaterialInstance _skeletalmesh 0 (Rendering|Material|GetMaterial _skeletalmesh 0) "None" :!class /Script/Engine.PrimitiveComponent))
  (Variables|Default|SetWheatMaterial _returnvalue)
  (Variables|Default|SetScale (.scale (Transformation|GetRelativeTransform (Variables|Default|GetSceneComp)))))

(event EventOnFullyWateredBP
  (bind _returnvalue (Math|Random|RandomFloatinRange 2.7 3.5))
  (bind _seedlingmesh (Variables|Default|GetSeedlingMesh))
  (bind _output_get (Variables|Default|SetScale (Math|Vector|MakeVector _returnvalue _returnvalue _returnvalue)))
  ;[1 1 1] On Fully Watered
  (bind (_direction _seedling _scale) (Timeline|Timeline_0 Play)
    (:Update
      (Transformation|SetActorRelativeScale3D (* _scale _output_get))
      (Transformation|SetRelativeScale3D (Variables|Default|GetSeedlingMesh) (Math|Vector|MakeVector 0.0 0.0 _seedling)))
    (:Finished
      (Rendering|SetVisibility _seedlingmesh false false)
      (Collision|SetCollisionEnabled _seedlingmesh "NoCollision"))))

(event EventOnSpawnHealthy
  ;[1 1 1] Healthy Spawn - Ground
  (bind _scale (Timeline|SpawnAnim Play)
    (:Update
      (Transformation|SetActorRelativeScale3D (* _scale (Variables|Default|GetScale))))))

(event EventOnSpawnUnhealthy
  ;[1 1 1] UnHealthy Spawn
  (Components|Animation|PlayAnimation (Variables|Default|GetSkeletalMesh) "/Game/Meshes/Plants/Wheat/Wheat_Seedling_02_Anim_Shrivel.Wheat_Seedling_02_Anim_Shrivel" false)
  (bind (_direction _size _color) (Timeline|Shrivel Play)
    (:Update
      (Rendering|Material|SetVectorParameterValue (Variables|Default|GetWheatMaterial) "Top Color" _color :!class /Script/Engine.MaterialInstanceDynamic)
      (Transformation|SetActorRelativeScale3D (* _size (Variables|Default|GetScale))))
    (:Finished
      (Class|CWheatSpawnable|SetReadytoDestroy true))))

(fn ConstructionScript)