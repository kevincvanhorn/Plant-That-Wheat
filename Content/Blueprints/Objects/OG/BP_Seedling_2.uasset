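; BP_Seedling_2 is a wheat seedling actor that plays a scale-based spawn animation when play begins.
; BeginPlay creates a dynamic material from the skeletal mesh and caches its scale, which the SpawnAnim timeline multiplies to drive actor scale.
; An alternate shrivel branch, with a skeletal animation and a timeline for top color and size, is switched off by a hardcoded false condition.
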(event EventBeginPlay
  (bind _skeletalmeshcomponent (Variables|SkeletalMeshActor|GetSkeletalMeshComponent))
  (bind _returnvalue (Rendering|Material|CreateDynamicMaterialInstance _skeletalmeshcomponent 0 (Rendering|Material|GetMaterial _skeletalmeshcomponent 0) "None" :!class /Script/Engine.PrimitiveComponent))
  (Variables|Default|SetWheatMaterial _returnvalue)
  (Variables|Default|SetScale (.scale (Transformation|GetRelativeTransform (Variables|SkeletalMeshActor|GetSkeletalMeshComponent))))
  (if false
    (Components|Animation|PlayAnimation (Variables|SkeletalMeshActor|GetSkeletalMeshComponent) "/Game/Meshes/Grass/Wheat/Wheat_Seedling_02_Anim_Shrivel.Wheat_Seedling_02_Anim_Shrivel" false)
    (bind (_direction _size _color) (Timeline|Shrivel Play)
      (:Update
        (Rendering|Material|SetVectorParameterValue (Variables|Default|GetWheatMaterial) "Top Color" _color :!class /Script/Engine.MaterialInstanceDynamic)
        (Transformation|SetActorRelativeScale3D (* _size (Variables|Default|GetScale)))))
    (else
      ;[1 1 1] Healthy Spawn - Ground
      (bind _scale (Timeline|SpawnAnim Play)
        (:Update
          (Transformation|SetActorRelativeScale3D (* _scale (Variables|Default|GetScale))))))))

(event Collision|EventActorBeginOverlap
  (params (OtherActor :type Actor%20Object%20Reference)))

(event EventTick
  (params (DeltaSeconds :type Float%20%28single-precision%29)))

(fn ConstructionScript)