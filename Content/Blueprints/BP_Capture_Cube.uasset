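; Scene capture actor that orients itself by quadrant toward the player and accumulates its capture into a persistent render target.
; Each tick it tests the player's direction; on a quadrant change it rotates, rebuilds its orthonormal basis and switches to that quadrant's render target.
; A dynamic material draws into RT_Persistent every tick, while MPC_Capture shares capture size and basis vectors with materials.
; MoveCapture is never called, and debug trace and print remain active.
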(event Custom|OnChangeQuadrant
  (bind _scenecapture (Variables|Default|GetSceneCapture))
  (CallFunction|UpdateLocalRotation)
  (bind _returnvalue (Class|CCaptureCube|GetRenderTargetbyIndex (Math|Conversions|ToInteger(Byte) (Variables|Default|GetQuadrant))))
  (Variables|/Script/Engine.SceneCaptureComponent2D|SetTextureTarget _scenecapture _returnvalue)
  (Rendering|Material|SetTextureParameterValue (Variables|Default|GetDrawMaterial) "RT_Texture" (Variables|/Script/Engine.SceneCaptureComponent2D|GetTextureTarget _scenecapture)))

(event EventBeginPlay
  (Rendering|Material|SetScalarParameterValue "/Game/Materials/Other/MPC_Capture.MPC_Capture" "CaptureSize" (Variables|/Script/Engine.SceneCaptureComponent2D|GetOrthoWidth (Variables|Default|GetSceneCapture)) :!class /Script/Engine.KismetMaterialLibrary)
  (Transformation|SetActorRotation "0, 0, 0")
  (bind _returnvalue (Rendering|Material|CreateDynamicMaterialInstance "/Game/Materials/Other/Mat_DrawToPersistent.Mat_DrawToPersistent" "None" :!class /Script/Engine.KismetMaterialLibrary))
  (Variables|Default|SetDrawMaterial _returnvalue)
  (CallFunction|ClearRenderTargets)
  (CallFunction|UpdateLocalRotation))

(event EventTick
  (params (DeltaSeconds :type Float%20%28single-precision%29))
  (CallFunction|CheckPlayerChunk)
  (CallFunction|DrawtoPersistent))

(fn ConstructionScript)

(fn DrawtoPersistent
  (Rendering|DrawMaterialtoRenderTarget "/Game/Core/RenderTargets/RT_Persistent.RT_Persistent" (Variables|Default|GetDrawMaterial)))

(fn MoveCapture
  (bind _returnvalue (Game|Player|GetPlayerPawn 0))
  (bind _returnvalue_2 (Transformation|GetActorLocation _returnvalue))
  (Variables|Default|SetMoveOffset (- (Math|Vector2D|MakeVector2D (Math|Vector|DotProduct _returnvalue_2 (Variables|Default|GetOrthonormalX)) (Math|Vector|DotProduct _returnvalue_2 (Variables|Default|GetOrthonormalY))) (Math|Vector2D|MakeVector2D (Math|Vector|DotProduct (Variables|Default|GetLastLocation) (Variables|Default|GetOrthonormalX)) (Math|Vector|DotProduct (Variables|Default|GetLastLocation) (Variables|Default|GetOrthonormalY)))))
  (Variables|Default|SetLastLocation _returnvalue_2))

(fn UpdateLocalRotation
  (Class|CCaptureCube|CreateOrthonormalBasis)
  (Rendering|Material|SetVectorParameterValue "/Game/Materials/Other/MPC_Capture.MPC_Capture" "CaptureVectorX" (Math|Conversions|ToLinearColor(Vector) (Variables|Default|GetOrthonormalX)) :!class /Script/Engine.KismetMaterialLibrary)
  (Rendering|Material|SetVectorParameterValue "/Game/Materials/Other/MPC_Capture.MPC_Capture" "CaptureVectorY" (Math|Conversions|ToLinearColor(Vector) (Variables|Default|GetOrthonormalY)) :!class /Script/Engine.KismetMaterialLibrary)
  (Rendering|Material|SetVectorParameterValue "/Game/Materials/Other/MPC_Capture.MPC_Capture" "CaptureVectorZ" (Math|Conversions|ToLinearColor(Vector) (Variables|Default|GetOrthonormalZ)) :!class /Script/Engine.KismetMaterialLibrary))

(fn CheckPlayerChunk
  (bind _returnvalue (Game|Player|GetPlayerPawn 0))
  (bind _returnvalue_2 (Transformation|GetActorLocation))
  (bind _returnvalue_3 (Transformation|GetActorRightVector))
  (bind _returnvalue_4 (Transformation|GetActorLocation _returnvalue))
  (bind _returnvalue_5 (- _returnvalue_4 _returnvalue_2))
  (bind _returnvalue_6 (Math|Rotator|MakeRotfromZY _returnvalue_5 _returnvalue_3))
  (Collision|LineTraceByChannel _returnvalue_2 (+ _returnvalue_2 (* (Transformation|GetActorUpVector) 5e+03)) "TraceTypeQuery1" false 0 "ForOneFrame")
  (bind _returnvalue_7 (Class|CCaptureCube|SetCaptureOrientation _returnvalue_6))
  (Development|PrintString (Utilities|String|ToString(Rotator) _returnvalue_6) true true "(R=0.000000,G=0.660000,B=1.000000,A=1.000000)" 6.0)
  (if _returnvalue_7
    ;[1 1 1] On Change of Quadrant
    (Transformation|SetActorRotation (Variables|Default|GetOrientation))
    (CallFunction|OnChangeQuadrant)))

(fn ClearRenderTargets
  (Rendering|ClearRenderTarget2D "/Game/Core/RenderTargets/RT_Capture.RT_Capture")
  (Rendering|ClearRenderTarget2D "/Game/Core/RenderTargets/RT_Persistent.RT_Persistent"))