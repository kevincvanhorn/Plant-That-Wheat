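; Cube-oriented capture actor that bakes a hole mask into render targets, choosing the target by the quadrant the player is in.
; Each tick it derives an orientation from the direction to the player, and on a quadrant change rotates and pushes its rebuilt orthonormal axes to MPC_Capture.
; It then draws Mat_RT_Holes into that quadrant's render target.
; MoveCapture computes player movement in the local 2D basis but is not called here.
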(event Custom|OnPlaceSphereMask
  (CallFunction|CheckPlayerChunk)
  (CallFunction|BakeHole))

(event Custom|OnChangeQuadrant
  (CallFunction|UpdateLocalRotation))

(event EventTick
  (params (DeltaSeconds :type Float%20%28single-precision%29))
  (CallFunction|OnPlaceSphereMask))

(event EventBeginPlay
  (Class|CCaptureCube|CreateOrthonormalBasis)
  (Rendering|Material|CreateDynamicMaterialInstance "/Game/Materials/Planet/PDesert/Sand/RT_Approach/Mat_Holes.Mat_Holes" "None" :!class /Script/Engine.KismetMaterialLibrary))

(fn ConstructionScript)

(fn MoveCapture
  (bind _returnvalue (Game|Player|GetPlayerPawn 0))
  (bind _returnvalue_2 (Transformation|GetActorLocation _returnvalue))
  (Variables|Default|SetMoveOffset (- (Math|Vector2D|MakeVector2D (Math|Vector|DotProduct _returnvalue_2 (Variables|Default|GetOrthonormalX)) (Math|Vector|DotProduct _returnvalue_2 (Variables|Default|GetOrthonormalY))) (Math|Vector2D|MakeVector2D (Math|Vector|DotProduct (Variables|Default|GetLastLocation) (Variables|Default|GetOrthonormalX)) (Math|Vector|DotProduct (Variables|Default|GetLastLocation) (Variables|Default|GetOrthonormalY)))))
  (Variables|Default|SetLastLocation _returnvalue_2))

(fn UpdateLocalRotation
  (bind _orthonormalx (Variables|Default|GetOrthonormalX))
  (bind _orthonormaly (Variables|Default|GetOrthonormalY))
  (bind _orthonormalz (Variables|Default|GetOrthonormalZ))
  (Class|CCaptureCube|CreateOrthonormalBasis)
  (Rendering|Material|SetVectorParameterValue "/Game/Materials/Other/MPC_Capture.MPC_Capture" "CaptureVectorX" (Math|Conversions|ToLinearColor(Vector) _orthonormalx) :!class /Script/Engine.KismetMaterialLibrary)
  (Rendering|Material|SetVectorParameterValue "/Game/Materials/Other/MPC_Capture.MPC_Capture" "CaptureVectorY" (Math|Conversions|ToLinearColor(Vector) _orthonormaly) :!class /Script/Engine.KismetMaterialLibrary)
  (Rendering|Material|SetVectorParameterValue "/Game/Materials/Other/MPC_Capture.MPC_Capture" "CaptureVectorZ" (Math|Conversions|ToLinearColor(Vector) _orthonormalz) :!class /Script/Engine.KismetMaterialLibrary)
  (Development|PrintString (Utilities|String|ToString(Vector) _orthonormalx))
  (Development|PrintString (Utilities|String|ToString(Vector) _orthonormaly))
  (Development|PrintString (Utilities|String|ToString(Vector) _orthonormalz)))

(fn CheckPlayerChunk
  (bind _returnvalue (Transformation|GetActorLocation))
  (Collision|LineTraceByChannel _returnvalue (+ _returnvalue (* (Transformation|GetActorUpVector) 5e+03)) "TraceTypeQuery1" false 0 "ForOneFrame")
  (bind _returnvalue_2 (Class|CCaptureCube|SetCaptureOrientation (Math|Rotator|MakeRotfromZY (- (Transformation|GetActorLocation (Game|Player|GetPlayerPawn 0)) _returnvalue) (Transformation|GetActorRightVector))))
  (if _returnvalue_2
    ;[1 1 1] On Change of Quadrant
    (Transformation|SetActorRotation (Variables|Default|GetOrientation))
    (CallFunction|OnChangeQuadrant)))

(fn BakeHole
  (bind _returnvalue (Class|CCaptureCube|GetRenderTargetbyIndex (Math|Conversions|ToInteger(Byte) (Variables|Default|GetQuadrant))))
  (Rendering|DrawMaterialtoRenderTarget _returnvalue "/Game/Materials/Planet/PDesert/Sand/RT_Approach/Mat_RT_Holes.Mat_RT_Holes"))