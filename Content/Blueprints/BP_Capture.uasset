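; Scene capture actor that maintains a persistent render target around the player, rotating in place so its up axis points at the player.
; Each tick it publishes its orthonormal basis to MPC_Capture and projects player movement onto that basis as a 2D offset.
; A dynamic material draws into RT_Persistent using that offset, normalized by ortho width.
; The older world-space move with pixel snapping is disconnected.
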(event EventBeginPlay
  (Rendering|Material|SetScalarParameterValue "/Game/Materials/MPC_Capture.MPC_Capture" "CaptureSize" (Variables|/Script/Engine.SceneCaptureComponent2D|GetOrthoWidth (Variables|Default|GetSceneCapture)) :!class /Script/Engine.KismetMaterialLibrary)
  (bind _returnvalue (Rendering|Material|CreateDynamicMaterialInstance "/Game/Materials/Mat_DrawToPersistent.Mat_DrawToPersistent" "None" :!class /Script/Engine.KismetMaterialLibrary))
  (Variables|Default|SetDrawMaterial _returnvalue)
  (Rendering|ClearRenderTarget2D "/Game/Core/RenderTargets/RT_Capture.RT_Capture")
  (Rendering|ClearRenderTarget2D "/Game/Core/RenderTargets/RT_Persistent.RT_Persistent")
  (CallFunction|UpdateLocalRotation)
  (Variables|Default|SetLastRotation (Transformation|GetActorRotation))
  (Variables|Default|SetLastLocation (Transformation|GetActorLocation (Game|Player|GetPlayerPawn 0))))

(event EventTick
  (params (DeltaSeconds :type Float%20%28single-precision%29))
  (bind _returnvalue (Transformation|GetActorLocation))
  (Variables|Default|SetLastRotation (Transformation|GetActorRotation))
  (Transformation|SetActorRotation (Math|Rotator|MakeRotfromZY (- (Transformation|GetActorLocation (Game|Player|GetPlayerPawn 0)) _returnvalue) (Transformation|GetActorRightVector)))
  (Collision|LineTraceByChannel _returnvalue (+ _returnvalue (* (Transformation|GetActorUpVector) 5e+03)) "TraceTypeQuery1" false 0 "ForOneFrame")
  (CallFunction|UpdateLocalRotation)
  (CallFunction|MoveCapture)
  (CallFunction|DrawtoPersistent))

(fn ConstructionScript)

(fn DrawtoPersistent
  (bind _scenecapture (Variables|Default|GetSceneCapture))
  (bind _moveoffset (Variables|Default|GetMoveOffset))
  (bind _orthowidth (Variables|/Script/Engine.SceneCaptureComponent2D|GetOrthoWidth _scenecapture))
  (bind _returnvalue (/ _moveoffset _orthowidth))
  (Rendering|Material|SetVectorParameterValue (Variables|Default|GetDrawMaterial) "Offset" (Utilities|Struct|MakeLinearColor (.x _returnvalue) (.y _returnvalue) 0.0 1.0) :!class /Script/Engine.MaterialInstanceDynamic)
  (Rendering|DrawMaterialtoRenderTarget "/Game/Core/RenderTargets/RT_Persistent.RT_Persistent" (Variables|Default|GetDrawMaterial)))

(fn MoveCapture
  (bind _returnvalue (Game|Player|GetPlayerPawn 0))
  (bind _returnvalue_2 (Transformation|GetActorLocation _returnvalue))
  (Variables|Default|SetMoveOffset (- (Math|Vector2D|MakeVector2D (Math|Vector|DotProduct _returnvalue_2 (Variables|Default|GetOrthonormalX)) (Math|Vector|DotProduct _returnvalue_2 (Variables|Default|GetOrthonormalY))) (Math|Vector2D|MakeVector2D (Math|Vector|DotProduct (Variables|Default|GetLastLocation) (Variables|Default|GetOrthonormalX)) (Math|Vector|DotProduct (Variables|Default|GetLastLocation) (Variables|Default|GetOrthonormalY)))))
  (Variables|Default|SetLastLocation _returnvalue_2))

(fn UpdateLocalRotation
  (Class|CCapture|CreateOrthonormalBasis)
  (Rendering|Material|SetVectorParameterValue "/Game/Materials/MPC_Capture.MPC_Capture" "CaptureVectorX" (Math|Conversions|ToLinearColor(Vector) (Variables|Default|GetOrthonormalX)) :!class /Script/Engine.KismetMaterialLibrary)
  (Rendering|Material|SetVectorParameterValue "/Game/Materials/MPC_Capture.MPC_Capture" "CaptureVectorY" (Math|Conversions|ToLinearColor(Vector) (Variables|Default|GetOrthonormalY)) :!class /Script/Engine.KismetMaterialLibrary)
  (Rendering|Material|SetVectorParameterValue "/Game/Materials/MPC_Capture.MPC_Capture" "CaptureVectorZ" (Math|Conversions|ToLinearColor(Vector) (Variables|Default|GetOrthonormalZ)) :!class /Script/Engine.KismetMaterialLibrary))