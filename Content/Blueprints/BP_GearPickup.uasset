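; BP_GearPickup is a gear pickup that dissolves and removes itself when it overlaps an objective.
; BeginPlay creates a dynamic material instance from the mesh's first material.
; OnObjectiveOverlap plays a timeline that drives that material's "Dissolve Amount" parameter.
; When the timeline finishes, the gear calls ExternalDropMoveable to drop itself as a moveable, then destroys the actor.
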(event EventBeginPlay
  (bind _meshcomponent (Variables|Default|GetMeshComponent))
  (bind _returnvalue (Rendering|Material|CreateDynamicMaterialInstance _meshcomponent 0 (Rendering|Material|GetMaterial _meshcomponent 0) "None" :!class /Script/Engine.PrimitiveComponent))
  (Variables|Default|SetDissolveMaterial _returnvalue))

(event Collision|EventActorBeginOverlap
  (params (OtherActor :type Actor%20Object%20Reference)))

(event EventTick
  (params (DeltaSeconds :type Float%20%28single-precision%29)))

(event EventOnObjectiveOverlap
  (bind _dissolve (Timeline|Dissolve%20Timeline Play)
    (:Update
      (Rendering|Material|SetScalarParameterValue (Variables|Default|GetDissolveMaterial) "Dissolve Amount" _dissolve :!class /Script/Engine.MaterialInstanceDynamic))
    (:Finished
      (Class|CMoveableActor|ExternalDropMoveable)
      (Actor|DestroyActor))))

(fn ConstructionScript)