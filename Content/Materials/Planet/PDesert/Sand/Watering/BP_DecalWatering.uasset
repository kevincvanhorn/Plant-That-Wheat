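; Decal actor for the watering effect on desert-planet sand, animating a wet mark each time OnStartAnimation fires.
; BeginPlay caches the decal's scale and gives it a dynamic material instance.
; The Anim_01 timeline drives damped opacity, color and actor scale with slight random size variation, then calls OnFinshAnimation.
; An older scale-only timeline, Anim, remains in the graph but never runs.
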(event EventBeginPlay
  (Variables|Default|SetScale (Variables|/Script/Engine.SceneComponent|GetRelativeScale3D (Variables|Default|GetDecal)))
  (bind _returnvalue (Rendering|Material|CreateDynamicMaterialInstance (Class|DecalComponent|GetDecalMaterial (Variables|Default|GetDecal)) "None" :!class /Script/Engine.KismetMaterialLibrary))
  (bind _output_get (Variables|Default|SetDecalMatInst _returnvalue))
  (Rendering|Components|Decal|SetDecalMaterial (Variables|Default|GetDecal) _output_get))

(event EventTick
  (params (DeltaSeconds :type Float%20%28single-precision%29)))

(event EventOnStartAnimation
  (bind _decalmatinst (Variables|Default|GetDecalMatInst))
  (Variables|Default|SetTempScale (* (Variables|Default|GetScale) (Math|Random|RandomFloatinRange 0.9 1.1)))
  (bind (_direction _opacity _scale _color) (Timeline|Anim_01 PlayFromStart)
    (:Update
      (Rendering|Material|SetScalarParameterValue _decalmatinst "Opacity" (* _opacity 0.15) :!class /Script/Engine.MaterialInstanceDynamic)
      (Transformation|SetActorRelativeScale3D (* (Variables|Default|GetTempScale) _scale))
      (Rendering|Material|SetVectorParameterValue _decalmatinst "Color" _color :!class /Script/Engine.MaterialInstanceDynamic))
    (:Finished
      (Class|CDecalActor|OnFinshAnimation))))

(fn ConstructionScript)