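; Planet desert sand actor that bakes a hole material into a render target and publishes its parameters to materials.
; The construction script calls Bake, which draws Mat_RT_Holes into RT_Hole_02.
; Bake also writes the referenced render target's width to MPC_Opacity and the actor's X scale to MPC_Planet as the scaled radius.
; It has no runtime logic, and the dynamic material instance setup is unconnected.
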(event EventBeginPlay)

(event Collision|EventActorBeginOverlap
  (params (OtherActor :type Actor%20Object%20Reference)))

(event EventTick
  (params (DeltaSeconds :type Float%20%28single-precision%29)))

(fn ConstructionScript
  (CallFunction|Bake))

(fn Bake
  (Rendering|DrawMaterialtoRenderTarget "/Game/Materials/Planet/PDesert/Sand/RT_Approach/RT_Hole_02.RT_Hole_02" "/Game/Materials/Planet/PDesert/Sand/RT_Approach/Mat_RT_Holes.Mat_RT_Holes")
  (Rendering|Material|SetScalarParameterValue "/Game/Materials/Planet/PDesert/MPC_Opacity.MPC_Opacity" "RT_Size" (Math|Conversions|ToFloat(Integer) (Variables|/Script/Engine.TextureRenderTarget2D|GetSizeX (Variables|Default|GetHole_RT_Reference))) :!class /Script/Engine.KismetMaterialLibrary)
  (Rendering|Material|SetScalarParameterValue "/Game/Materials/Foliage/MPC_Planet.MPC_Planet" "ScaledRadius" (.x (Transformation|GetActorScale3D)) :!class /Script/Engine.KismetMaterialLibrary))