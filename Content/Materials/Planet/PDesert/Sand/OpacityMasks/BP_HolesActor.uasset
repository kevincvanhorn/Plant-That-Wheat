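; Actor that feeds a list of hole locations to the Mat_Holes material on its static mesh, apparently for opacity-mask holes in desert sand.
; BeginPlay creates a tiny BP_HolesRT canvas render target, hands it HoleLocs, and binds it as the "Locations" texture of a dynamic material instance.
; Tick re-copies HoleLocs and redraws the target every frame, using the texture as a data channel into the shader.
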(event EventBeginPlay
  (Utilities|FlowControl|Sequence
    (:then_0
      (bind _returnvalue (CanvasRenderTarget2D|CreateCanvasRenderTarget2D "/Game/Materials/Planet/PDesert/Sand/OpacityMasks/BP_HolesRT.BP_HolesRT_C" 100 2))
      (bind _output_get (Variables|Default|SetBPHoles_RT _returnvalue))
      (bind _asbp_holes_rt (Utilities|Casting|CastToBP_HolesRT _output_get))
      (Variables|/Game/Materials/Planet/PDesert/Sand/OpacityMasks/BP_HolesRT.BP_HolesRT_C|SetHoleLocs_RT _asbp_holes_rt (Variables|Components|GetHoleLocs)))
    (:then_1
      (bind _returnvalue_2 (Rendering|Material|CreateDynamicMaterialInstance "/Game/Materials/Planet/PDesert/Sand/OpacityMasks/Mat_Holes.Mat_Holes" "None" :!class /Script/Engine.KismetMaterialLibrary))
      (Rendering|Material|SetTextureParameterValue _returnvalue_2 "Locations" _returnvalue)
      (Class|CanvasRenderTarget2D|UpdateResource _returnvalue)
      (Rendering|Material|SetMaterial (Variables|Default|GetStaticMesh) 0 _returnvalue_2))))

(event EventTick
  (params (DeltaSeconds :type Float%20%28single-precision%29))
  (bind _bpholes_rt (Variables|Default|GetBPHoles_RT))
  (bind _asbp_holes_rt (Utilities|Casting|CastToBP_HolesRT _bpholes_rt))
  (Variables|/Game/Materials/Planet/PDesert/Sand/OpacityMasks/BP_HolesRT.BP_HolesRT_C|SetHoleLocs_RT _asbp_holes_rt (Variables|Components|GetHoleLocs))
  (Class|CanvasRenderTarget2D|UpdateResource _bpholes_rt))

(fn ConstructionScript)